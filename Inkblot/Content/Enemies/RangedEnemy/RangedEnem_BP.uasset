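; Ranged enemy character that turns to face the player and fires projectiles on a cooldown, paired with the RAngedEnemAIC AI controller.
; While LookingAtPlayer is set, Tick rotates the capsule toward player 0.
; Shoot spawns BP_Projectile at ShootingPoint, clears CanShoot and starts a timer that restores it after ShootCooldown.
; Both changes to CanShoot are passed to the controller through SetShoot.
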(event Custom|Shoot
  (Development|PrintString "Shhot")
  (Variables|Default|SetCanShoot false)
  (Game|SpawnActorfromClass "/Game/Enemies/RangedEnemy/BP_Projectile.BP_Projectile_C" (Transformation|GetWorldTransform (Variables|Default|GetShootingPoint)) "Undefined" "MultiplyWithRoot" 0 0)
  (Utilities|Time|SetTimerbyEvent (delegate Custom|ReserShoot) (Variables|Default|GetShootCooldown))
  (bind _asranged_enem_aic (Utilities|Casting|CastToRAngedEnemAIC (Pawn|GetController)))
  (Default|SetShoot _asranged_enem_aic (Variables|Default|GetCanShoot)))

(event Custom|ReserShoot
  (Variables|Default|SetCanShoot true)
  (bind _asranged_enem_aic (Utilities|Casting|CastToRAngedEnemAIC (Pawn|GetController)))
  (Default|SetShoot _asranged_enem_aic (Variables|Default|GetCanShoot)))

(event EventBeginPlay
  (|CallParentFunction)
  (Variables|Default|SetAIControllerClass "/Game/Enemies/RangedEnemy/RAngedEnemAIC.RAngedEnemAIC_C"))

(event Collision|EventActorBeginOverlap
  (params (OtherActor :type Actor%20Object%20Reference)))

(event EventTick
  (params (DeltaSeconds :type Float%20%28single-precision%29))
  (bind _capsulecomponent (Variables|Default|GetCapsuleComponent))
  (if (Variables|Default|GetLookingAtPlayer)
    (Transformation|SetWorldRotation _capsulecomponent (Math|Rotator|FindLookatRotation (Transformation|GetWorldLocation _capsulecomponent) (Transformation|GetActorLocation (Game|GetPlayerCharacter 0))) false false)))

(fn ConstructionScript
  (|CallParentFunction))