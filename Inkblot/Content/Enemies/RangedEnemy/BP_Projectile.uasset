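; BP_Projectile is a ranged-enemy projectile that damages BP_TopDownCharacter on contact.
; On BeginPlay, a LifeSpan timer is set to destroy the actor.
; Sphere1 overlaps apply fixed damage to the character and destroy the projectile, pass through Dummy actors, and destroy it on any other actor except itself.
; Debug prints remain, and a Shoot function, not called in this Blueprint, spawns another BP_Projectile at its own location.
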(event OnComponentHit(Sphere1)
  (params (HitComponent :type Primitive%20Component%20Object%20Reference) (OtherActor :type Actor%20Object%20Reference) (OtherComp :type Primitive%20Component%20Object%20Reference) (NormalImpulse :type Vector :default "0, 0, 0") (Hit :type Hit%20Result%20Structure%20%28by%20ref%29)))

(event OnComponentBeginOverlap(Sphere1)
  (params (OverlappedComponent :type Primitive%20Component%20Object%20Reference) (OtherActor :type Actor%20Object%20Reference) (OtherComp :type Primitive%20Component%20Object%20Reference) (OtherBodyIndex :type Integer) (bFromSweep :type Boolean) (SweepResult :type Hit%20Result%20Structure%20%28by%20ref%29))
  (Development|PrintString (Utilities|GetDisplayName OtherActor))
  (if (not (== OtherActor self))
    (bind _asbp_top_down_character (Utilities|Casting|CastToBP_TopDownCharacter OtherActor)
      (:then
        (Game|Damage|ApplyDamage _asbp_top_down_character 1e+01 0 0)
        (Actor|DestroyActor))
      (:CastFailed
        (Utilities|Casting|CastToDummy OtherActor
          (:CastFailed
            (Actor|DestroyActor)))))))

(event Custom|Destrot
  (Development|PrintString "Hello")
  (Actor|DestroyActor))

(event EventBeginPlay
  (Utilities|Time|SetTimerbyEvent (delegate Custom|Destrot) (Variables|Default|GetLifeSpan)))

(fn ConstructionScript)

(fn Shoot
  (Game|SpawnActorfromClass "BP_Projectile_C" (Math|Conversions|ToTransform(Vector) (Transformation|GetActorLocation)) "Undefined" "MultiplyWithRoot" 0 0))